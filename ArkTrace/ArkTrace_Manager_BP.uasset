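; ArkTrace manager that holds the mod's live event tracing state and log, and handles its script command.
; Construction reads the global tracing toggle from the game mode INI.
; Trace entries submitted on the server are broadcast through a notify dispatcher, then stored newest-first for bulk retrieval.
; A game mode custom-event binding gives cheat-permitted players the ArkTrace_CommLayer buff when the command arrives.
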(event `self.ReceiveBeginPlay`
  (bind _asshootergamemode (cast `ShooterGameMode` (`GameplayStatics.GetGameMode`)))
  (add `self.OnActorCustomEvent` _asshootergamemode (delegate `ActorCustomEventSignature__DelegateSignature_Event`))
  ;[1 1 1] Live Event Tracing log (Do not mimic this method this is to prevent circular dependancies. the macro cannot be used in the negotiator bluprint.)
  (bind _bistracingenabled (`self.GetLiveEventTraceMode`))
  (if _bistracingenabled
    (`self.Submit Live Event Trace Log to Negotiator` (make `/Game/Mods/ArkTrace/ArkTrace/FArkTrace_LiveEventTraceEntry` (`KismetMathLibrary.UtcNow`) "NewEnumerator0" self null "ArkTrace command bound"))))

(event `ActorCustomEventSignature__DelegateSignature_Event` :!signature `self.OnActorCustomEvent`
  (params (EventCustomName :type Name) (EventCustomString :type String) (InstigatorActor :type "Actor Object Reference"))
  (switch `string` EventCustomString
    (:`ScriptCommand ArkTrace [ModName]`
      (bind _returnvalue (`self.GetOwnerController` InstigatorActor))
      (bind _asshooterplayercontroller (cast `ShooterPlayerController` _returnvalue))
      (bind _asshootergamemode (cast `ShooterGameMode` (`GameplayStatics.GetGameMode`)))
      (bind _returnvalue_2 (`ShooterGameMode.IsPlayerAllowedToCheat` _asshootergamemode _asshooterplayercontroller))
      (if _returnvalue_2
        (`PrimalBuff.StaticAddBuff` "/Game/Mods/ArkTrace/ArkTrace/ArkTrace_CommLayer.ArkTrace_CommLayer_C" (`ShooterPlayerController.GetPlayerCharacter` _asshooterplayercontroller) null null true)))))

(fn `Get Bulk Live Event Trace Logs`
  (returns (LiveEventTraceLogs :type "Array of /Game/Mods/ArkTrace/ArkTrace/FArkTrace_LiveEventTraceEntry Structure"))
  (return (`self.LiveEventTraceLogs`)))

(fn `GetLiveEventTraceMode`
  (returns (bIsTracingEnabled :type Boolean))
  (return (`self.bIsGlobalLiveEventTracingEnabled`)))

(fn `Submit Live Event Trace Log to Negotiator`
  (params (LiveEventTraceEntry :type "/Game/Mods/ArkTrace/ArkTrace/FArkTrace_LiveEventTraceEntry Structure"))
  ;[1 1 1] Dispatch new live event trace then add to the log
  (`/Engine/EditorBlueprintResources/ActorMacros.SwitchNetAuthority`
    (:`DedicatedServer`
      _)
    (:`PlayerServer`
      _))
  (`self.BPNotifyLiveEventTraceEntry` LiveEventTraceEntry)
  (`KismetArrayLibrary.Array_Insert` (`self.LiveEventTraceLogs`) LiveEventTraceEntry)
  (return))

(fn `UserConstructionScript`
  (`|ExecutionSequence`
    (:`then_0`
      ;[1 1 1] Initialize Global Live Event Tracing Status
      (bind _asshootergamemode (cast `ShooterGameMode` (`GameplayStatics.GetGameMode`)))
      (`ShooterGameMode.InitOptionBool` _asshootergamemode "" "ArkTrace" "EnableGlobalLiveEventTracing" true)
      (bind _returnvalue (`ShooterGameMode.GetBoolOptionIni` _asshootergamemode "ArkTrace" "EnableGlobalLiveEventTracing"))
      (set `self.bIsGlobalLiveEventTracingEnabled` _returnvalue)
      ;[1 1 1] Live Event Tracing log (Do not mimic this method this is to prevent circular dependancies. the macro cannot be used in the negotiator bluprint.)
      (bind _bistracingenabled (`self.GetLiveEventTraceMode`))
      (if _bistracingenabled
        (`self.Submit Live Event Trace Log to Negotiator` (make `/Game/Mods/ArkTrace/ArkTrace/FArkTrace_LiveEventTraceEntry` (`KismetMathLibrary.UtcNow`) "NewEnumerator0" self _asshootergamemode "Global event trace state collected from INI"))))
    (:`then_1`
      ;[1 1 1] Live Event Tracing log (Do not mimic this method this is to prevent circular dependancies. the macro cannot be used in the negotiator bluprint.)
      (bind _bistracingenabled_2 (`self.GetLiveEventTraceMode`))
      (if _bistracingenabled_2
        (`self.Submit Live Event Trace Log to Negotiator` (make `/Game/Mods/ArkTrace/ArkTrace/FArkTrace_LiveEventTraceEntry` (`KismetMathLibrary.UtcNow`) "NewEnumerator0" self null "ArkTrace contructor completed"))))))